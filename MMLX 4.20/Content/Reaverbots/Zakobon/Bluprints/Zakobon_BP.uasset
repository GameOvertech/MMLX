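; Zakobon Reaverbot enemy that can be targeted, takes damage and drops items on death.
; Any hit on its capsule removes a fixed amount of health, with debug prints and no check on what hit it.
; At zero health it clears IsAlive, spawns Spawn_items_BP at its transform, plays an explosion sound and destroys itself.
; Targeting functions report IsAlive as targetability and show or hide the Widget on selection changes.
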(event `self.ReceiveBeginPlay`)

(event `self.Capsule.OnComponentHit`
  (params (HitComponent :type "PrimitiveComponent Object Reference") (OtherActor :type "Actor Object Reference") (OtherComp :type "PrimitiveComponent Object Reference") (NormalImpulse :type "Vector Structure") (Hit :type "HitResult Structure (by ref)"))
  (`KismetSystemLibrary.PrintString` "OUCHIES!!!!")
  (bind _output_get (set `self.ZakobonHealth` (- (`self.ZakobonHealth`) 6)))
  (`KismetSystemLibrary.PrintString` (`KismetStringLibrary.Conv_IntToString` _output_get))
  (if (<= (`self.ZakobonHealth`) 0)
    (set `self.isAlive` false)
    (`/Engine/EditorBlueprintResources/StandardMacros.DoOnce` false
      (:`Completed`
        (`|SpawnActorFromClass` "/Game/Blueprints/Zenny/Spawn_items_BP.Spawn_items_BP_C" (`self.GetTransform`) "Undefined" "OverrideRootScale" null null)
        (`GameplayStatics.PlaySound2D` "/Game/Audio/SFX/sfx_reaverbot/sfx-explosion1.sfx-explosion1" 1.0 1.0 0.0 null null)
        (`self.K2_DestroyActor`)))))

(event `self.StaticMeshComponent.OnComponentBeginOverlap`
  (params (OverlappedComponent :type "PrimitiveComponent Object Reference") (OtherActor :type "Actor Object Reference") (OtherComp :type "PrimitiveComponent Object Reference") (OtherBodyIndex :type Integer) (bFromSweep :type Boolean) (SweepResult :type "HitResult Structure (by ref)")))

(event `self.StaticMeshComponent.OnComponentHit`
  (params (HitComponent :type "PrimitiveComponent Object Reference") (OtherActor :type "Actor Object Reference") (OtherComp :type "PrimitiveComponent Object Reference") (NormalImpulse :type "Vector Structure") (Hit :type "HitResult Structure (by ref)")))

(fn `IsTargetable`
  (returns (`return value` :type Boolean))
  (return (`self.isAlive`)))

(fn `OnDeselected`
  (returns (DummyValue :type Boolean))
  (`SceneComponent.SetHiddenInGame` (`self.Widget`) true false)
  (return false))

(fn `OnSelected`
  (returns (DummyValue :type Boolean))
  (`SceneComponent.SetHiddenInGame` (`self.Widget`) false false)
  (return false))

(fn `UserConstructionScript`)