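; Destructible, targetable refractor container that drops zenny and cubes when destroyed.
; AnyDamage lowers BoxHP with hurt sound and explosion effect; at zero, Tick spawns Spawn_items_BP with drop amounts and probabilities, then destroys the actor.
; Box hits drain a separate RefractorContainerHealth that only clears IsAlive, without triggering drops or destruction.
; IsTargetable returns IsAlive, and selection callbacks show or hide the Widget.
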(event `self.ReceiveAnyDamage`
  (params (Damage :type "Float (single-precision)") (DamageType :type "DamageType Object Reference") (InstigatedBy :type "Controller Object Reference") (DamageCauser :type "Actor Object Reference"))
  ;[1 1 1] Taking Damage
  (bind _output_get (set `self.boxHP` (- (`self.boxHP`) (`KismetMathLibrary.FFloor` Damage))))
  (`KismetSystemLibrary.PrintString` (`KismetStringLibrary.Conv_IntToString` _output_get))
  (`GameplayStatics.PlaySound2D` "/Game/Audio/SFX/sfx_reaverbot/sfx-reaverhurt1.sfx-reaverhurt1" 1.0 1.0 0.0 null null)
  (`GameplayStatics.SpawnEmitterAtLocation` "/Game/StarterContent/Particles/P_Explosion.P_Explosion" (`self.K2_GetActorLocation`)))

(event `self.ReceiveTick`
  (params (DeltaSeconds :type "Float (single-precision)"))
  ;[1 1 1] Alive Check
  (if (<= (`KismetMathLibrary.Conv_IntToDouble` (`self.boxHP`)) 0.0)
    (set `self.isAlive` false)
    (if (not (`self.isAlive`))
      (`KismetSystemLibrary.PrintString` "kill me")
      (`/Engine/EditorBlueprintResources/StandardMacros.DoOnce` false
        (:`Completed`
          (bind _returnvalue (`|SpawnActorFromClass` "/Game/Blueprints/Zenny/Spawn_items_BP.Spawn_items_BP_C" (`self.GetTransform`) "Undefined" "OverrideRootScale" null null))
          (set `/Game/Blueprints/Zenny/Spawn_items_BP.amount_of_zenny_to_drop` (`self.amount_of_zenny_to_drop`) _returnvalue)
          (set `/Game/Blueprints/Zenny/Spawn_items_BP.amount_of_cubes_to_drop` (`self.amount_of_cubes_to_drop`) _returnvalue)
          (set `/Game/Blueprints/Zenny/Spawn_items_BP.Probability_of_pale` 0 _returnvalue)
          (set `/Game/Blueprints/Zenny/Spawn_items_BP.probability_of_green` 0 _returnvalue)
          (set `/Game/Blueprints/Zenny/Spawn_items_BP.probabilty_of_pink` 1 _returnvalue)
          (set `/Game/Blueprints/Zenny/Spawn_items_BP.probabilty_of_purple` 2 _returnvalue)
          (`/Game/Blueprints/Zenny/Spawn_items_BP.spawn_things_event` _returnvalue)
          (`GameplayStatics.PlaySound2D` "/Game/Audio/SFX/sfx_reaverbot/sfx-explosion1.sfx-explosion1" 1.0 1.0 0.0 null null)
          (`self.K2_DestroyActor`))))))

(event `self.ReceiveBeginPlay`
  (set `self.isAlive` true)
  (set `self.boxHP` 150))

(event `self.Box.OnComponentHit`
  (params (HitComponent :type "PrimitiveComponent Object Reference") (OtherActor :type "Actor Object Reference") (OtherComp :type "PrimitiveComponent Object Reference") (NormalImpulse :type "Vector Structure") (Hit :type "HitResult Structure (by ref)"))
  (`KismetSystemLibrary.PrintString` "SHOW ME THE ZENNY!!!")
  (bind _output_get (set `self.RefractorContainerHealth` (- (`self.RefractorContainerHealth`) 12)))
  (`KismetSystemLibrary.PrintString` (`KismetStringLibrary.Conv_IntToString` _output_get))
  (if (<= (`self.RefractorContainerHealth`) 0)
    (set `self.isAlive` false)))

(fn `IsTargetable`
  (returns (`return value` :type Boolean))
  (return (`self.isAlive`)))

(fn `OnDeselected`
  (returns (DummyValue :type Boolean))
  (`SceneComponent.SetHiddenInGame` (`self.Widget`) true false)
  (return false))

(fn `OnSelected`
  (returns (DummyValue :type Boolean))
  (`SceneComponent.SetHiddenInGame` (`self.Widget`) false false)
  (return false))

(fn `UserConstructionScript`)