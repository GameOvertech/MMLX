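; Tower elevator actor that the player rides up and down by pressing Interact inside its trigger box.
; Overlap with a component tagged MegamanCapsule toggles the actor's input and its interact flag.
; Each press plays sounds and flip-flops a timeline between play and reverse, driving the elevator root's relative Z.
; The actor disables its own input while the timeline updates and re-enables it when finished.
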(event `self.ReceiveBeginPlay`
  (set `self.Interact` false))

(event `self.ElevatorTriggerBox.OnComponentBeginOverlap`
  (params (OverlappedComponent :type "PrimitiveComponent Object Reference") (OtherActor :type "Actor Object Reference") (OtherComp :type "PrimitiveComponent Object Reference") (OtherBodyIndex :type Integer) (bFromSweep :type Boolean) (SweepResult :type "HitResult Structure (by ref)"))
  (if (`ActorComponent.ComponentHasTag` OtherComp "MegamanCapsule")
    (`self.EnableInput` (`GameplayStatics.GetPlayerController` 0))
    (set `self.Interact` true)))

(event `self.ReceiveActorBeginOverlap`
  (params (OtherActor :type "Actor Object Reference")))

(event `InputAction|Interact`
  (params (Key :type "Key Structure"))
  (bind _returnvalue (`GameplayStatics.GetPlayerController` 0))
  (:`Pressed`
    (if (`self.Interact`)
      (`GameplayStatics.PlaySound2D` "/Game/Audio/SFX/sfx_general/sfx-cursor-select1.sfx-cursor-select1")
      (`GameplayStatics.PlaySound2D` "/Game/Audio/SFX/sfx_general/sfx-elevator-Long.sfx-elevator-Long")
      (`/Engine/EditorBlueprintResources/StandardMacros.FlipFlop`
        (:`A`
          (bind (_direction _verticalmotion) (`Timeline|ElevatorAnimation` :!label _label)
            (:`Update`
              (`self.DisableInput` _returnvalue)
              (`SceneComponent.K2_SetRelativeTransform` (`self.ElevatorROOT`) (`KismetMathLibrary.MakeTransform` (`KismetMathLibrary.MakeVector` 0.0 0.0 (.z (.location (`KismetMathLibrary.MakeTransform` (`KismetMathLibrary.MakeVector` 0.0 0.0 _verticalmotion)))))) false false))
            (:`Finished`
              (`self.EnableInput` _returnvalue))))
        (:`B`
          (goto _label :!via `Reverse`))))))

(event `self.ElevatorTriggerBox.OnComponentEndOverlap`
  (params (OverlappedComponent :type "PrimitiveComponent Object Reference") (OtherActor :type "Actor Object Reference") (OtherComp :type "PrimitiveComponent Object Reference") (OtherBodyIndex :type Integer))
  (if (`ActorComponent.ComponentHasTag` OtherComp "MegamanCapsule")
    (`self.DisableInput` (`GameplayStatics.GetPlayerController` 0))
    (set `self.Interact` false)))

(fn `UserConstructionScript`)