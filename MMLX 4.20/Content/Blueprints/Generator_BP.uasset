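; Destructible generator objective that shields the level's force fields until the generators are destroyed.
; Every hit on its capsule subtracts fixed HP and prints feedback; at zero it plays an explosion sound and destroys itself.
; It then checks the ThirdPersonGameMode's GeneratorsDestroyed flag and, if set, removes two ForceField_BP actors found by class lookup.
; Tick calls the game mode's GeneratorCounter every frame.
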(event `self.ReceiveTick`
  (params (DeltaSeconds :type "Float (single-precision)"))
  (bind _asthird_person_game_mode (cast `/Game/ThirdPersonBP/Blueprints/ThirdPersonGameMode` (`GameplayStatics.GetGameMode`))
    (:`then`
      (`/Game/ThirdPersonBP/Blueprints/ThirdPersonGameMode.GeneratorCounter` _asthird_person_game_mode))
    (:`CastFailed`
      (`KismetSystemLibrary.PrintString` "Destroy the Generators!"))))

(event `self.Capsule.OnComponentHit`
  (params (HitComponent :type "PrimitiveComponent Object Reference") (OtherActor :type "Actor Object Reference") (OtherComp :type "PrimitiveComponent Object Reference") (NormalImpulse :type "Vector Structure") (Hit :type "HitResult Structure (by ref)"))
  (`KismetSystemLibrary.PrintString` "SHEILDS DAMAGED!!!!")
  (bind _output_get (set `self.GeneratorHP` (- (`self.GeneratorHP`) 6)))
  (`KismetSystemLibrary.PrintString` (`KismetStringLibrary.Conv_IntToString` _output_get))
  (if (<= (`self.GeneratorHP`) 0)
    (`GameplayStatics.PlaySound2D` "/Game/Audio/SFX/sfx_reaverbot/sfx-explosion1.sfx-explosion1")
    (`self.K2_DestroyActor`)
    (bind _asthird_person_game_mode (cast `/Game/ThirdPersonBP/Blueprints/ThirdPersonGameMode` (`GameplayStatics.GetGameMode`)))
    (if (`/Game/ThirdPersonBP/Blueprints/ThirdPersonGameMode.GeneratorsDestroyed` _asthird_person_game_mode)
      (`|ExecutionSequence`
        (:`then_0`
          (bind _outactors (`GameplayStatics.GetAllActorsOfClass` "/Game/Blueprints/ForceField_BP.ForceField_BP_C"))
          (bind _asforce_field_bp (cast `/Game/Blueprints/ForceField_BP` (`|GetArrayItem` _outactors 1)))
          (`/Game/Blueprints/ForceField_BP.DestroyForceField` _asforce_field_bp))
        (:`then_1`
          (bind _outactors_2 (`GameplayStatics.GetAllActorsOfClass` "/Game/Blueprints/ForceField_BP.ForceField_BP_C"))
          (bind _asforce_field_bp_2 (cast `/Game/Blueprints/ForceField_BP` (`|GetArrayItem` _outactors_2)))
          (`/Game/Blueprints/ForceField_BP.DestroyForceField` _asforce_field_bp_2))))))

(fn `UserConstructionScript`)