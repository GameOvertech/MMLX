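; One-shot booby trap that springs when anything overlaps its Box, sealing a trap door and releasing Mirumijee spawns.
; A timeline sinks the Scene component along Z, then shuts the first TrapDoor_BP found in the level.
; If that succeeds, it calls MirumijeeSPAWN on six Mirumijee_BP actors, picked by hard-coded GetAllActorsOfClass indices.
; Debug strings print at each stage and when the door cast fails.
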(event `self.Box.OnComponentBeginOverlap`
  (params (OverlappedComponent :type "PrimitiveComponent Object Reference") (OtherActor :type "Actor Object Reference") (OtherComp :type "PrimitiveComponent Object Reference") (OtherBodyIndex :type Integer) (bFromSweep :type Boolean) (SweepResult :type "HitResult Structure (by ref)"))
  (`/Engine/EditorBlueprintResources/StandardMacros.DoOnce` false
    (:`Completed`
      (bind (_direction _verticalsink) (`Timeline|BoobyTrap`)
        (:`Update`
          (`SceneComponent.K2_SetRelativeTransform` (`self.Scene`) (`KismetMathLibrary.MakeTransform` (`KismetMathLibrary.MakeVector` 0.0 0.0 (.z (.location (`KismetMathLibrary.MakeTransform` (`KismetMathLibrary.MakeVector` 0.0 0.0 _verticalsink)))))) false false))
        (:`Finished`
          (`KismetSystemLibrary.PrintString` "Yove Been Boobed")
          (bind _outactors (`GameplayStatics.GetAllActorsOfClass` "/Game/Blueprints/TrapDoor_BP.TrapDoor_BP_C"))
          (bind _astrap_door_bp (cast `/Game/Blueprints/TrapDoor_BP` (`|GetArrayItem` _outactors))
            (:`then`
              (`/Game/Blueprints/TrapDoor_BP.TrapDoorShut` _astrap_door_bp)
              (`KismetSystemLibrary.PrintString` "TRAPPED!!!!")
              (`|ExecutionSequence`
                (:`then_0`
                  (bind _outactors_2 (`GameplayStatics.GetAllActorsOfClass` "/Game/Reaverbots/Mirumijee/Blueprints/Mirumijee_BP.Mirumijee_BP_C"))
                  (bind _asmirumijee_bp (cast `/Game/Reaverbots/Mirumijee/Blueprints/Mirumijee_BP` (`|GetArrayItem` _outactors_2)))
                  (`/Game/Reaverbots/Mirumijee/Blueprints/Mirumijee_BP.MirumijeeSPAWN` _asmirumijee_bp)
                  (`KismetSystemLibrary.PrintString` "KILL THE WABBIT!!!"))
                (:`then_1`
                  (bind _outactors_3 (`GameplayStatics.GetAllActorsOfClass` "/Game/Reaverbots/Mirumijee/Blueprints/Mirumijee_BP.Mirumijee_BP_C"))
                  (bind _asmirumijee_bp_2 (cast `/Game/Reaverbots/Mirumijee/Blueprints/Mirumijee_BP` (`|GetArrayItem` _outactors_3 1)))
                  (`/Game/Reaverbots/Mirumijee/Blueprints/Mirumijee_BP.MirumijeeSPAWN` _asmirumijee_bp_2)
                  (`KismetSystemLibrary.PrintString` "KILL THE WABBIT!!!"))
                (:`then_2`
                  (bind _outactors_4 (`GameplayStatics.GetAllActorsOfClass` "/Game/Reaverbots/Mirumijee/Blueprints/Mirumijee_BP.Mirumijee_BP_C"))
                  (bind _asmirumijee_bp_3 (cast `/Game/Reaverbots/Mirumijee/Blueprints/Mirumijee_BP` (`|GetArrayItem` _outactors_4 2)))
                  (`/Game/Reaverbots/Mirumijee/Blueprints/Mirumijee_BP.MirumijeeSPAWN` _asmirumijee_bp_3)
                  (`KismetSystemLibrary.PrintString` "KILL THE WABBIT!!!"))
                (:`then_3`
                  (bind _outactors_5 (`GameplayStatics.GetAllActorsOfClass` "/Game/Reaverbots/Mirumijee/Blueprints/Mirumijee_BP.Mirumijee_BP_C"))
                  (bind _asmirumijee_bp_4 (cast `/Game/Reaverbots/Mirumijee/Blueprints/Mirumijee_BP` (`|GetArrayItem` _outactors_5 3)))
                  (`/Game/Reaverbots/Mirumijee/Blueprints/Mirumijee_BP.MirumijeeSPAWN` _asmirumijee_bp_4)
                  (`KismetSystemLibrary.PrintString` "KILL THE WABBIT!!!"))
                (:`then_4`
                  (bind _outactors_6 (`GameplayStatics.GetAllActorsOfClass` "/Game/Reaverbots/Mirumijee/Blueprints/Mirumijee_BP.Mirumijee_BP_C"))
                  (bind _asmirumijee_bp_5 (cast `/Game/Reaverbots/Mirumijee/Blueprints/Mirumijee_BP` (`|GetArrayItem` _outactors_6 4)))
                  (`/Game/Reaverbots/Mirumijee/Blueprints/Mirumijee_BP.MirumijeeSPAWN` _asmirumijee_bp_5)
                  (`KismetSystemLibrary.PrintString` "KILL THE WABBIT!!!"))
                (:`then_5`
                  (bind _outactors_7 (`GameplayStatics.GetAllActorsOfClass` "/Game/Reaverbots/Mirumijee/Blueprints/Mirumijee_BP.Mirumijee_BP_C"))
                  (bind _asmirumijee_bp_6 (cast `/Game/Reaverbots/Mirumijee/Blueprints/Mirumijee_BP` (`|GetArrayItem` _outactors_7 5)))
                  (`/Game/Reaverbots/Mirumijee/Blueprints/Mirumijee_BP.MirumijeeSPAWN` _asmirumijee_bp_6)
                  (`KismetSystemLibrary.PrintString` "KILL THE WABBIT!!!"))))
            (:`CastFailed`
              (`KismetSystemLibrary.PrintString` "FAILED!"))))))))

(fn `UserConstructionScript`)