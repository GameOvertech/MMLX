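; Buster gun plasma projectile that damages tagged enemies it overlaps.
; A CollisionCheck overlap with an "Enemy" actor prints its name, then tries a sequence of per-class casts, applying BusterPlasmaDamage and destroying itself on a match.
; The Generator_BP branch leaves the damage target unset.
; The range timeout only starts on a non-enemy overlap, waiting RangeDuration before spawning an explosion and destroying the projectile.
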(event `self.ReceiveActorBeginOverlap`
  (params (OtherActor :type "Actor Object Reference")))

(event `self.ReceiveTick`
  (params (DeltaSeconds :type "Float (single-precision)")))

(event `self.CollisionCheck.OnComponentBeginOverlap`
  (params (OverlappedComponent :type "PrimitiveComponent Object Reference") (OtherActor :type "Actor Object Reference") (OtherComp :type "PrimitiveComponent Object Reference") (OtherBodyIndex :type Integer) (bFromSweep :type Boolean) (SweepResult :type "HitResult Structure (by ref)"))
  (if (`self.ActorHasTag` OtherActor "Enemy")
    (`KismetSystemLibrary.PrintString` (`KismetSystemLibrary.GetDisplayName` OtherActor))
    (`|ExecutionSequence`
      (:`then_0`
        ;[1 1 1] If can be casted to the type of enemy then run these
        (bind _aszakobon (cast `/Game/Reaverbots/Zakobon/Bluprints/Zakobon` OtherActor))
        (`GameplayStatics.ApplyDamage` _aszakobon (`KismetMathLibrary.Conv_IntToDouble` (`self.BusterPlasmaDamage`)))
        (`self.K2_DestroyActor`))
      (:`then_1`
        (bind _asmirumijee_bp (cast `/Game/Reaverbots/Mirumijee/Blueprints/Mirumijee_BP` OtherActor))
        (`GameplayStatics.ApplyDamage` _asmirumijee_bp (`KismetMathLibrary.Conv_IntToDouble` (`self.BusterPlasmaDamage`)))
        (`self.K2_DestroyActor`))
      (:`then_2`
        (bind _ashanmuru_doll_bp (cast `/Game/Reaverbots/HanmuruDoll/Blueprints/HanmuruDoll_BP` OtherActor))
        (`GameplayStatics.ApplyDamage` _ashanmuru_doll_bp (`KismetMathLibrary.Conv_IntToDouble` (`self.BusterPlasmaDamage`)))
        (`self.K2_DestroyActor`))
      (:`then_3`
        (bind _ascannam_bp (cast `/Game/Reaverbots/Cannam/Blueprints/Cannam_BP` OtherActor))
        (`GameplayStatics.ApplyDamage` _ascannam_bp (`KismetMathLibrary.Conv_IntToDouble` (`self.BusterPlasmaDamage`)))
        (`self.K2_DestroyActor`))
      (:`then_4`
        (cast `/Game/Blueprints/Actor/Generator_BP` OtherActor)
        (`GameplayStatics.ApplyDamage` null (`KismetMathLibrary.Conv_IntToDouble` (`self.BusterPlasmaDamage`)))
        (`self.K2_DestroyActor`))
      (:`then_5`
        (bind _asrefractor_container_bp (cast `/Game/Blueprints/Actor/RefractorContainer_BP` OtherActor))
        (`GameplayStatics.ApplyDamage` _asrefractor_container_bp (`KismetMathLibrary.Conv_IntToDouble` (`self.BusterPlasmaDamage`)))
        (`self.K2_DestroyActor`))
      (:`then_6`
        (bind _asparent_enemy_moving_bp2 (cast `/Game/Reaverbots/parent_enemy_moving_BP2` OtherActor))
        (`GameplayStatics.ApplyDamage` _asparent_enemy_moving_bp2 (`KismetMathLibrary.Conv_IntToDouble` (`self.BusterPlasmaDamage`)))
        (`self.K2_DestroyActor`)))
    (else
      ;[1 1 1] Range timeout
      (`KismetSystemLibrary.Delay` (`self.RangeDuration`))
      (`GameplayStatics.SpawnEmitterAtLocation` "/Game/StarterContent/Particles/P_Explosion.P_Explosion" (`self.K2_GetActorLocation`))
      (`self.K2_DestroyActor`))))

(fn `UserConstructionScript`)