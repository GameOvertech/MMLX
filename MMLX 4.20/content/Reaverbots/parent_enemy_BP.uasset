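; Base Reaverbot enemy Blueprint that handles health, destruction, loot drops and player targeting.
; AnyDamage subtracts floored damage with sound and explosion effects, while any capsule hit removes a fixed amount of HP.
; Tick polls HP and on death spawns a larger explosion, creates a Spawn_items_BP actor to drop Zenny and cubes, then destroys itself.
; Targeting functions report alive state and toggle a widget when selected or deselected.
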(event `self.ReceiveAnyDamage`
  (params (Damage :type "Float (single-precision)") (DamageType :type "DamageType Object Reference") (InstigatedBy :type "Controller Object Reference") (DamageCauser :type "Actor Object Reference"))
  ;[1 1 1] Taking Damage
  (set `self.EnemyHP` (- (`self.EnemyHP`) (`KismetMathLibrary.FFloor` Damage)))
  (`GameplayStatics.PlaySound2D` "/Game/Audio/SFX/sfx_reaverbot/sfx-reaverhurt1.sfx-reaverhurt1" 1.0 1.0 0.0 null null)
  (`GameplayStatics.SpawnEmitterAtLocation` "/Game/StarterContent/Particles/P_Explosion.P_Explosion" (`self.K2_GetActorLocation`)))

(event `self.ReceiveBeginPlay`
  (set `self.isAlive` true))

(event `self.ReceiveTick`
  (params (DeltaSeconds :type "Float (single-precision)"))
  ;[1 1 1] Alive Check
  (if (<= (`KismetMathLibrary.Conv_IntToDouble` (`self.EnemyHP`)) 0.0)
    (set `self.isAlive` false)
    ;[1 1 1] If destroyed
    (if (not (`self.isAlive`))
      (`GameplayStatics.SpawnEmitterAtLocation` "/Game/StarterContent/Particles/P_Explosion.P_Explosion" (`self.K2_GetActorLocation`) (struct) (3.0 3.0 3.0))
      (`KismetSystemLibrary.PrintString` "kill me")
      (`/Engine/EditorBlueprintResources/StandardMacros.DoOnce` false
        (:`Completed`
          (bind _returnvalue (`|SpawnActorFromClass` "/Game/Blueprints/Zenny/Spawn_items_BP.Spawn_items_BP_C" (`self.GetTransform`) "Undefined" "OverrideRootScale" null null))
          (set `/Game/Blueprints/Zenny/Spawn_items_BP.amount_of_zenny_to_drop` (`self.amount_of_zenny_to_drop`) _returnvalue)
          (set `/Game/Blueprints/Zenny/Spawn_items_BP.amount_of_cubes_to_drop` (`self.amount_of_cubes_to_drop`) _returnvalue)
          (`/Game/Blueprints/Zenny/Spawn_items_BP.spawn_things_event` _returnvalue)
          (`GameplayStatics.PlaySound2D` "/Game/Audio/SFX/sfx_reaverbot/sfx-explosion1.sfx-explosion1" 1.0 1.0 0.0 null null)
          (`self.K2_DestroyActor`))))))

(event `self.Capsule.OnComponentHit`
  (params (HitComponent :type "PrimitiveComponent Object Reference") (OtherActor :type "Actor Object Reference") (OtherComp :type "PrimitiveComponent Object Reference") (NormalImpulse :type "Vector Structure") (Hit :type "HitResult Structure (by ref)"))
  ;[1 1 1] Touched by Mega
  (`KismetSystemLibrary.PrintString` (`KismetStringLibrary.Concat_StrStr` "What is hitting the enemy" (`KismetStringLibrary.Conv_ObjectToString` OtherActor)))
  (`KismetSystemLibrary.PrintString` "Mega's Touching me!!!")
  (bind _output_get (set `self.EnemyHP` (- (`self.EnemyHP`) 6)))
  (`KismetSystemLibrary.PrintString` (`KismetStringLibrary.Conv_IntToString` _output_get))
  (if (<= (`self.EnemyHP`) 0)
    (set `self.isAlive` false)))

(fn `IsTargetable`
  (returns (`return value` :type Boolean))
  (return (`self.isAlive`)))

(fn `OnDeselected`
  (returns (DummyValue :type Boolean))
  (`SceneComponent.SetHiddenInGame` (`self.Widget`) true false)
  (return false))

(fn `OnSelected`
  (returns (DummyValue :type Boolean))
  (`SceneComponent.SetHiddenInGame` (`self.Widget`) false false)
  (return false))

(fn `UserConstructionScript`)