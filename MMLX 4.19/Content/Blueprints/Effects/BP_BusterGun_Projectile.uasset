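; Buster gun plasma projectile that damages actors tagged Enemy on overlap and destroys itself.
; A sequence of casts repeats health subtraction, hit effects and death explosion for each of six target classes.
; Mirumijee and Generator kills check game mode flags to shut the trap door or drop two force fields.
; Overlapping anything untagged starts a RangeDuration delay, then the projectile explodes and is destroyed.
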(event `self.ReceiveActorBeginOverlap`
  (params (OtherActor :type "Actor Object Reference")))

(event `self.ReceiveTick`
  (params (DeltaSeconds :type "Float (single-precision)")))

(event `self.CollisionCheck.OnComponentBeginOverlap`
  (params (OverlappedComponent :type "PrimitiveComponent Object Reference") (OtherActor :type "Actor Object Reference") (OtherComp :type "PrimitiveComponent Object Reference") (OtherBodyIndex :type Integer) (bFromSweep :type Boolean) (SweepResult :type "HitResult Structure (by ref)"))
  (if (`self.ActorHasTag` OtherActor "Enemy")
    (`self.K2_DestroyActor`)
    (`|ExecutionSequence`
      (:`then_0`
        (bind _aszakobon_bp (cast `/Game/Reaverbots/Zakobon/Bluprints/Zakobon_BP` OtherActor))
        (bind _output_get (set `/Game/Reaverbots/Zakobon/Bluprints/Zakobon_BP.ZakobonHealth` (- (`/Game/Reaverbots/Zakobon/Bluprints/Zakobon_BP.ZakobonHealth` _aszakobon_bp) (`self.BusterPlasmaDamage`)) _aszakobon_bp))
        (`KismetSystemLibrary.PrintString` (`KismetStringLibrary.Conv_IntToString` _output_get))
        (`GameplayStatics.PlaySound2D` "/Game/Audio/SFX/sfx_reaverbot/sfx-reaverhurt1.sfx-reaverhurt1")
        (`GameplayStatics.SpawnEmitterAtLocation` "/Game/StarterContent/Particles/P_Explosion.P_Explosion" (`self.K2_GetActorLocation`))
        (if (<= (`KismetMathLibrary.Conv_IntToDouble` (`/Game/Reaverbots/Zakobon/Bluprints/Zakobon_BP.ZakobonHealth` _aszakobon_bp)) 0.0)
          (`GameplayStatics.SpawnEmitterAtLocation` "/Game/StarterContent/Particles/P_Explosion.P_Explosion" (`self.K2_GetActorLocation` _aszakobon_bp) (struct) (3.0 3.0 3.0))
          (`GameplayStatics.PlaySound2D` "/Game/Audio/SFX/sfx_reaverbot/sfx-explosion1.sfx-explosion1")
          (`self.K2_DestroyActor` _aszakobon_bp)))
      (:`then_1`
        (bind _asmirumijee_bp (cast `/Game/Reaverbots/Mirumijee/Blueprints/Mirumijee_BP` OtherActor))
        (bind _output_get_2 (set `/Game/Reaverbots/Mirumijee/Blueprints/Mirumijee_BP.MirumijeeHealth` (- (`/Game/Reaverbots/Mirumijee/Blueprints/Mirumijee_BP.MirumijeeHealth` _asmirumijee_bp) (`self.BusterPlasmaDamage`)) _asmirumijee_bp))
        (`KismetSystemLibrary.PrintString` (`KismetStringLibrary.Conv_IntToString` _output_get_2))
        (`GameplayStatics.PlaySound2D` "/Game/Audio/SFX/sfx_reaverbot/sfx-reaverhurt1.sfx-reaverhurt1")
        (`GameplayStatics.SpawnEmitterAtLocation` "/Game/StarterContent/Particles/P_Explosion.P_Explosion" (`self.K2_GetActorLocation`))
        (if (<= (`KismetMathLibrary.Conv_IntToDouble` (`/Game/Reaverbots/Mirumijee/Blueprints/Mirumijee_BP.MirumijeeHealth` _asmirumijee_bp)) 0.0)
          (`GameplayStatics.SpawnEmitterAtLocation` "/Game/StarterContent/Particles/P_Explosion.P_Explosion" (`self.K2_GetActorLocation` _asmirumijee_bp) (struct) (3.0 3.0 3.0))
          (`GameplayStatics.PlaySound2D` "/Game/Audio/SFX/sfx_reaverbot/sfx-explosion1.sfx-explosion1")
          (`self.K2_DestroyActor` _asmirumijee_bp)
          (`self.K2_DestroyActor`)
          (bind _asthird_person_game_mode (cast `/Game/ThirdPersonBP/Blueprints/ThirdPersonGameMode` (`GameplayStatics.GetGameMode`)))
          (if (`/Game/ThirdPersonBP/Blueprints/ThirdPersonGameMode.MirumijeeAllDead` _asthird_person_game_mode)
            (bind _outactors (`GameplayStatics.GetAllActorsOfClass` "/Game/Blueprints/Actor/TrapDoor_BP.TrapDoor_BP_C"))
            (bind _astrap_door_bp (cast `/Game/Blueprints/Actor/TrapDoor_BP` (`|GetArrayItem` _outactors)))
            (`/Game/Blueprints/Actor/TrapDoor_BP.TrapDoorShut` _astrap_door_bp))))
      (:`then_2`
        (bind _ashanmuru_doll_bp (cast `/Game/Reaverbots/HanmuruDoll/Blueprints/HanmuruDoll_BP` OtherActor))
        (bind _output_get_3 (set `/Game/Reaverbots/HanmuruDoll/Blueprints/HanmuruDoll_BP.HanmuruHealth` (- (`/Game/Reaverbots/HanmuruDoll/Blueprints/HanmuruDoll_BP.HanmuruHealth` _ashanmuru_doll_bp) (`self.BusterPlasmaDamage`)) _ashanmuru_doll_bp))
        (`KismetSystemLibrary.PrintString` (`KismetStringLibrary.Conv_IntToString` _output_get_3))
        (`GameplayStatics.PlaySound2D` "/Game/Audio/SFX/sfx_reaverbot/sfx-reaverhurt1.sfx-reaverhurt1")
        (`GameplayStatics.SpawnEmitterAtLocation` "/Game/StarterContent/Particles/P_Explosion.P_Explosion" (`self.K2_GetActorLocation`))
        (if (<= (`KismetMathLibrary.Conv_IntToDouble` (`/Game/Reaverbots/HanmuruDoll/Blueprints/HanmuruDoll_BP.HanmuruHealth` _ashanmuru_doll_bp)) 0.0)
          (`GameplayStatics.SpawnEmitterAtLocation` "/Game/StarterContent/Particles/P_Explosion.P_Explosion" (`self.K2_GetActorLocation`) (struct) (3.0 3.0 3.0))
          (`GameplayStatics.PlaySound2D` "/Game/Audio/SFX/sfx_reaverbot/sfx-explosion1.sfx-explosion1")
          (`self.K2_DestroyActor` _ashanmuru_doll_bp)
          (`self.K2_DestroyActor`)))
      (:`then_3`
        (bind _ascannam_bp (cast `/Game/Reaverbots/Cannam/Blueprints/Cannam_BP` OtherActor))
        (bind _output_get_4 (set `/Game/Reaverbots/Cannam/Blueprints/Cannam_BP.CannamHP` (- (`/Game/Reaverbots/Cannam/Blueprints/Cannam_BP.CannamHP` _ascannam_bp) (`self.BusterPlasmaDamage`)) _ascannam_bp))
        (`KismetSystemLibrary.PrintString` (`KismetStringLibrary.Conv_IntToString` _output_get_4))
        (`GameplayStatics.PlaySound2D` "/Game/Audio/SFX/sfx_reaverbot/sfx-reaverhurt1.sfx-reaverhurt1")
        (`GameplayStatics.SpawnEmitterAtLocation` "/Game/StarterContent/Particles/P_Explosion.P_Explosion" (`self.K2_GetActorLocation`))
        (if (<= (`KismetMathLibrary.Conv_IntToDouble` (`/Game/Reaverbots/Cannam/Blueprints/Cannam_BP.CannamHP` _ascannam_bp)) 0.0)
          (`GameplayStatics.SpawnEmitterAtLocation` "/Game/StarterContent/Particles/P_Explosion.P_Explosion" (`self.K2_GetActorLocation`) (struct) (3.0 3.0 3.0))
          (`GameplayStatics.PlaySound2D` "/Game/Audio/SFX/sfx_reaverbot/sfx-explosion1.sfx-explosion1")
          (`self.K2_DestroyActor` _ascannam_bp)
          (`self.K2_DestroyActor`)))
      (:`then_4`
        (bind _asgenerator_bp (cast `/Game/Blueprints/Actor/Generator_BP` OtherActor))
        (bind _output_get_5 (set `/Game/Blueprints/Actor/Generator_BP.GeneratorHP` (- (`/Game/Blueprints/Actor/Generator_BP.GeneratorHP` _asgenerator_bp) (`self.BusterPlasmaDamage`)) _asgenerator_bp))
        (`KismetSystemLibrary.PrintString` (`KismetStringLibrary.Conv_IntToString` _output_get_5))
        (`GameplayStatics.PlaySound2D` "/Game/Audio/SFX/sfx_reaverbot/sfx-reaverhurt1.sfx-reaverhurt1")
        (`GameplayStatics.SpawnEmitterAtLocation` "/Game/StarterContent/Particles/P_Explosion.P_Explosion" (`self.K2_GetActorLocation`))
        (if (<= (`KismetMathLibrary.Conv_IntToDouble` (`/Game/Blueprints/Actor/Generator_BP.GeneratorHP` _asgenerator_bp)) 0.0)
          (`GameplayStatics.SpawnEmitterAtLocation` "/Game/StarterContent/Particles/P_Explosion.P_Explosion" (`self.K2_GetActorLocation`) (struct) (3.0 3.0 3.0))
          (`GameplayStatics.PlaySound2D` "/Game/Audio/SFX/sfx_reaverbot/sfx-explosion1.sfx-explosion1")
          (`self.K2_DestroyActor` _asgenerator_bp)
          (bind _asthird_person_game_mode_2 (cast `/Game/ThirdPersonBP/Blueprints/ThirdPersonGameMode` (`GameplayStatics.GetGameMode`)))
          (if (`/Game/ThirdPersonBP/Blueprints/ThirdPersonGameMode.GeneratorsDestroyed` _asthird_person_game_mode_2)
            (`|ExecutionSequence`
              (:`then_0`
                (bind _outactors_2 (`GameplayStatics.GetAllActorsOfClass` "/Game/Blueprints/Actor/ForceField_BP.ForceField_BP_C"))
                (`/Game/Blueprints/Actor/ForceField_BP.DestroyForceField` (`|GetArrayItem` _outactors_2 1)))
              (:`then_1`
                (bind _outactors_3 (`GameplayStatics.GetAllActorsOfClass` "/Game/Blueprints/Actor/ForceField_BP.ForceField_BP_C"))
                (`/Game/Blueprints/Actor/ForceField_BP.DestroyForceField` (`|GetArrayItem` _outactors_3)))))))
      (:`then_5`
        (bind _asrefractor_container_bp (cast `/Game/Blueprints/Actor/RefractorContainer_BP` OtherActor))
        (bind _output_get_6 (set `/Game/Blueprints/Actor/RefractorContainer_BP.RefractorContainerHealth` (- (`/Game/Blueprints/Actor/RefractorContainer_BP.RefractorContainerHealth` _asrefractor_container_bp) (`self.BusterPlasmaDamage`)) _asrefractor_container_bp))
        (`KismetSystemLibrary.PrintString` (`KismetStringLibrary.Conv_IntToString` _output_get_6))
        (`GameplayStatics.PlaySound2D` "/Game/Audio/SFX/sfx_reaverbot/sfx-reaverhurt1.sfx-reaverhurt1")
        (`GameplayStatics.SpawnEmitterAtLocation` "/Game/StarterContent/Particles/P_Explosion.P_Explosion" (`self.K2_GetActorLocation`))
        (if (<= (`KismetMathLibrary.Conv_IntToDouble` (`/Game/Blueprints/Actor/RefractorContainer_BP.RefractorContainerHealth` _asrefractor_container_bp)) 0.0)
          (`GameplayStatics.SpawnEmitterAtLocation` "/Game/StarterContent/Particles/P_Explosion.P_Explosion" (`self.K2_GetActorLocation`) (struct) (3.0 3.0 3.0))
          (`GameplayStatics.PlaySound2D` "/Game/Audio/SFX/sfx_reaverbot/sfx-explosion1.sfx-explosion1")
          (`self.K2_DestroyActor` _asrefractor_container_bp)
          (`self.K2_DestroyActor`))))
    (else
      (`KismetSystemLibrary.Delay` (`self.RangeDuration`))
      (`GameplayStatics.SpawnEmitterAtLocation` "/Game/StarterContent/Particles/P_Explosion.P_Explosion" (`self.K2_GetActorLocation`))
      (`self.K2_DestroyActor`))))

(fn `UserConstructionScript`)