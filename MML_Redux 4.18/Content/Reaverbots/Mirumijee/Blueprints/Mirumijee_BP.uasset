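; Mirumijee_BP is a Reaverbot enemy that drops in on spawn and can be destroyed by hits.
; MirumijeeSPAWN plays a one-time timeline that animates its relative height.
; Any capsule hit subtracts health; at zero it plays an explosion, destroys itself, and shuts the first TrapDoor_BP if the game mode reports all Mirumijees dead.
; Tick calls the game mode's MirumijeeCounter every frame.
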(event `self.ReceiveTick`
  (params (DeltaSeconds :type "Float (single-precision)"))
  (bind _asthird_person_game_mode (cast `/Game/ThirdPersonBP/Blueprints/ThirdPersonGameMode` (`GameplayStatics.GetGameMode`))
    (:`then`
      (`/Game/ThirdPersonBP/Blueprints/ThirdPersonGameMode.MirumijeeCounter` _asthird_person_game_mode))
    (:`CastFailed`
      (`KismetSystemLibrary.PrintString` "You Have Failed"))))

(event `self.Capsule.OnComponentHit`
  (params (HitComponent :type "PrimitiveComponent Object Reference") (OtherActor :type "Actor Object Reference") (OtherComp :type "PrimitiveComponent Object Reference") (NormalImpulse :type "Vector Structure") (Hit :type "HitResult Structure (by ref)"))
  (`KismetSystemLibrary.PrintString` "Ouchies")
  (bind _output_get (set `self.MirumijeeHealth` (- (`self.MirumijeeHealth`) 4)))
  (`KismetSystemLibrary.PrintString` (`KismetStringLibrary.Conv_IntToString` _output_get))
  (if (<= (`self.MirumijeeHealth`) 0)
    (`GameplayStatics.PlaySound2D` "/Game/Audio/SFX/sfx_reaverbot/sfx-explosion1.sfx-explosion1")
    (`self.K2_DestroyActor`)
    (bind _asthird_person_game_mode (cast `/Game/ThirdPersonBP/Blueprints/ThirdPersonGameMode` (`GameplayStatics.GetGameMode`)))
    (if (`/Game/ThirdPersonBP/Blueprints/ThirdPersonGameMode.MirumijeeAllDead` _asthird_person_game_mode)
      (bind _outactors (`GameplayStatics.GetAllActorsOfClass` "/Game/Blueprints/Actor/TrapDoor_BP.TrapDoor_BP_C"))
      (bind _astrap_door_bp (cast `/Game/Blueprints/Actor/TrapDoor_BP` (`|GetArrayItem` _outactors)))
      (`/Game/Blueprints/Actor/TrapDoor_BP.TrapDoorShut` _astrap_door_bp))))

(event `MirumijeeSPAWN`
  (`/Engine/EditorBlueprintResources/StandardMacros.DoOnce` false
    (:`Completed`
      (bind (_direction _newtrack_0) (`Timeline|MirumijeeFALL`)
        (:`Update`
          (`SceneComponent.K2_SetRelativeTransform` (`self.Mirumijee_Transform`) (`KismetMathLibrary.MakeTransform` (`KismetMathLibrary.MakeVector` 0.0 0.0 (.z (.location (`KismetMathLibrary.MakeTransform` (`KismetMathLibrary.MakeVector` 0.0 0.0 _newtrack_0)))))) false false))))))

(fn `UserConstructionScript`)