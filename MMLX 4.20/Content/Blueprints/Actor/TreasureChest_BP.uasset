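; Treasure chest actor whose lid opens, with sound, when the player presses Interact inside its trigger.
; Overlapping OpenTrigger enables player input and sets a proximity flag, then a DoOnce gates an OpenTreasure timeline that rolls the lid pivot.
; If the player has left when opening finishes, a second DoOnce prints a message, plays the close sound and runs the CloseTreasure timeline.
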(event `self.OpenTrigger.OnComponentBeginOverlap`
  (params (OverlappedComponent :type "PrimitiveComponent Object Reference") (OtherActor :type "Actor Object Reference") (OtherComp :type "PrimitiveComponent Object Reference") (OtherBodyIndex :type Integer) (bFromSweep :type Boolean) (SweepResult :type "HitResult Structure (by ref)"))
  (`self.EnableInput` (`GameplayStatics.GetPlayerController` 0))
  (set `self.NearTreasure` true)
  (if (and (`self.Interact`) (`self.NearTreasure`)) :!label _label
    (set `self.Interact` false)
    (`/Engine/EditorBlueprintResources/StandardMacros.DoOnce` false
      (:`Completed`
        (`GameplayStatics.PlaySound2D` "/Game/Audio/SFX/sfx_general/sfx-treasure-open1_Cue.sfx-treasure-open1_Cue")
        (bind (_direction _xrotate) (`Timeline|OpenTreasure`)
          (:`Update`
            (`SceneComponent.K2_SetRelativeTransform` (`self.TreasureTop_Pivot`) (`KismetMathLibrary.MakeTransform` (0.0 37.558105 49.872353) (`KismetMathLibrary.MakeRotator` (.roll (.rotation (`KismetMathLibrary.MakeTransform` (0.0 0.0 0.0) (`KismetMathLibrary.MakeRotator` _xrotate)))))) false false))
          (:`Finished`
            (if (not (`self.NearTreasure`))
              (`/Engine/EditorBlueprintResources/StandardMacros.DoOnce` false
                (:`Completed`
                  (`KismetSystemLibrary.PrintString` "Yay Treasure!")
                  (`GameplayStatics.PlaySound2D` "/Game/Audio/SFX/sfx_general/sfx-treasure-close1_Cue.sfx-treasure-close1_Cue")
                  (bind (_direction_2 _xrotate_2) (`Timeline|CloseTreasure`)
                    (:`Update`
                      (`SceneComponent.K2_SetRelativeTransform` (`self.TreasureTop_Pivot`) (`KismetMathLibrary.MakeTransform` (0.0 37.558105 49.872353) (`KismetMathLibrary.MakeRotator` (.roll (.rotation (`KismetMathLibrary.MakeTransform` (0.0 0.0 0.0) (`KismetMathLibrary.MakeRotator` _xrotate_2)))))) false false))))))))))
    (else
      (set `self.Interact` false))))

(event `InputAction|Interact`
  (params (Key :type "Key Structure"))
  (:`Pressed`
    (set `self.Interact` true)
    (goto _label)))

(event `self.OpenTrigger.OnComponentEndOverlap`
  (params (OverlappedComponent :type "PrimitiveComponent Object Reference") (OtherActor :type "Actor Object Reference") (OtherComp :type "PrimitiveComponent Object Reference") (OtherBodyIndex :type Integer))
  (set `self.NearTreasure` false))

(fn `UserConstructionScript`)