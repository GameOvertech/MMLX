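; Cannam Reaverbot actor that takes damage when hit and destroys itself when its health runs out.
; Any hit on CannamCollider subtracts a fixed amount from CannamHP, with no check on what struck it, and prints debug text with the remaining health.
; At zero or below it plays a 2D explosion sound and destroys the actor.
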(event `self.CannamCollider.OnComponentHit`
  (params (HitComponent :type "PrimitiveComponent Object Reference") (OtherActor :type "Actor Object Reference") (OtherComp :type "PrimitiveComponent Object Reference") (NormalImpulse :type "Vector Structure") (Hit :type "HitResult Structure (by ref)"))
  (`KismetSystemLibrary.PrintString` "OUCHIES!!!!")
  (bind _output_get (set `self.CannamHP` (- (`self.CannamHP`) 6)))
  (`KismetSystemLibrary.PrintString` (`KismetStringLibrary.Conv_IntToString` _output_get))
  (if (<= (`self.CannamHP`) 0)
    (`GameplayStatics.PlaySound2D` "/Game/Audio/SFX/sfx_reaverbot/sfx-explosion1.sfx-explosion1")
    (`self.K2_DestroyActor`)))

(fn `UserConstructionScript`)