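; GreenZenny_BP is a green Zenny currency pickup that scales up on BeginPlay and spins around its yaw every Tick.
; On actor overlap, it loops over the other actor's overlapping components and compares each to the player's ThirdPersonCharacter.
; A match prints a debug string, plays the pickup sound, adds 50 to the character's MegaZennyCount and destroys the pickup.
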(event `self.ReceiveBeginPlay`
  (`self.SetActorRelativeScale3D` (8.0 8.0 8.0)))

(event `self.ReceiveActorBeginOverlap`
  (params (OtherActor :type "Actor Object Reference"))
  (for _array_element (`self.GetOverlappingComponents` OtherActor)
    (if (== _array_element (cast `/Game/ThirdPersonBP/Blueprints/ThirdPersonCharacter` (`GameplayStatics.GetPlayerCharacter` 0) :!pure true))
      (`KismetSystemLibrary.PrintString` "yyyy")
      (`GameplayStatics.SpawnSoundAtLocation` "/Game/Audio/SFX/sfx_general/sfx-getzenny1.sfx-getzenny1" (`self.K2_GetActorLocation` self))
      (bind _asthird_person_character (cast `/Game/ThirdPersonBP/Blueprints/ThirdPersonCharacter` (`GameplayStatics.GetPlayerCharacter` 0)))
      (set `/Game/ThirdPersonBP/Blueprints/ThirdPersonCharacter.MegaZennyCount` (+ (`/Game/ThirdPersonBP/Blueprints/ThirdPersonCharacter.MegaZennyCount` _asthird_person_character) 50) _asthird_person_character)
      (`self.K2_DestroyActor`))))

(event `self.ReceiveTick`
  (params (DeltaSeconds :type "Float (single-precision)"))
  ;[1 1 1] Rotating Zenny
  (`self.K2_SetActorRotation` (`KismetMathLibrary.MakeRotator` (.roll (`self.K2_GetActorRotation` self)) (.pitch (`self.K2_GetActorRotation` self)) (+ (.yaw (`self.K2_GetActorRotation` self)) 2.0))))

(fn `UserConstructionScript`)