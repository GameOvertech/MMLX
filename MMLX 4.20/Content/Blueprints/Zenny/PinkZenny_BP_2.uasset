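; Pink Zenny pickup that adds 500 to the player character's MegaZennyCount when touched.
; On overlap with the player it plays a pickup sound at its location, increments the count on ThirdPersonCharacter and destroys itself.
; It enlarges itself on BeginPlay and spins around the yaw axis by a fixed step each tick, independent of delta time.
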(event `self.ReceiveBeginPlay`
  (`self.SetActorRelativeScale3D` (12.0 12.0 12.0)))

(event `self.ReceiveActorBeginOverlap`
  (params (OtherActor :type "Actor Object Reference"))
  (bind _returnvalue (`GameplayStatics.GetPlayerCharacter` 0))
  (if (== OtherActor _returnvalue)
    (`GameplayStatics.SpawnSoundAtLocation` "/Game/Audio/SFX/sfx_general/sfx-getzenny1.sfx-getzenny1" (`self.K2_GetActorLocation` self))
    (bind _asthird_person_character (cast `/Game/ThirdPersonBP/Blueprints/ThirdPersonCharacter` _returnvalue))
    (set `/Game/ThirdPersonBP/Blueprints/ThirdPersonCharacter.MegaZennyCount` (+ (`/Game/ThirdPersonBP/Blueprints/ThirdPersonCharacter.MegaZennyCount` _asthird_person_character) 500) _asthird_person_character)
    (`self.K2_DestroyActor`)))

(event `self.ReceiveTick`
  (params (DeltaSeconds :type "Float (single-precision)"))
  (`self.K2_SetActorRotation` (`KismetMathLibrary.MakeRotator` (.roll (`self.K2_GetActorRotation` self)) (.pitch (`self.K2_GetActorRotation` self)) (+ (.yaw (`self.K2_GetActorRotation` self)) 2.0))))

(fn `UserConstructionScript`)