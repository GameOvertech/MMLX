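; GreenZenny_BP is a spinning zenny pickup actor that scales itself up eightfold on BeginPlay and yaws a fixed step every tick.
; On overlap it searches the other actor's overlapping components for the player character's Xxx component and only prints a debug string.
; The collection logic (sound, adding 50 to the player's MegaZennyCount, self-destruct) is disconnected and never runs.
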(event `self.ReceiveBeginPlay`
  (`self.SetActorRelativeScale3D` (8.0 8.0 8.0)))

(event `self.ReceiveActorBeginOverlap`
  (params (OtherActor :type "Actor Object Reference"))
  (for _array_element (`self.GetOverlappingComponents` OtherActor)
    (if (== _array_element (`/Game/ThirdPersonBP/Blueprints/ThirdPersonCharacter.xxx` (cast `/Game/ThirdPersonBP/Blueprints/ThirdPersonCharacter` (`GameplayStatics.GetPlayerCharacter` 0) :!pure true)))
      (`KismetSystemLibrary.PrintString` "yyyy"))))

(event `self.ReceiveTick`
  (params (DeltaSeconds :type "Float (single-precision)"))
  (`self.K2_SetActorRotation` (`KismetMathLibrary.MakeRotator` (.roll (`self.K2_GetActorRotation` self)) (.pitch (`self.K2_GetActorRotation` self)) (+ (.yaw (`self.K2_GetActorRotation` self)) 2.0))))

(fn `UserConstructionScript`)