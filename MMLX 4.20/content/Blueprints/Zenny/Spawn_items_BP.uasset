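; Loot spawner actor that scatters zenny pickups and orange energy cubes, then destroys itself.
; spawn_things_event rolls a random zenny color per drop, then a per-color chance, so some drops yield nothing; cubes spawn in a fixed, configurable count.
; Each pickup spawns at a RandomLocInCircle transform and its mesh gets a DisperalSpread impulse to fling it outward.
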(event `spawn_things_event`
  ;[1 1 1] Zenny Drops
  (for _ (range 1 (+ (`self.amount_of_zenny_to_drop`) 1))
    (set `self.which_type_of_zenny` (`KismetMathLibrary.RandomIntegerInRange` 0 3))
    (switch `int` (`self.which_type_of_zenny`)
      (:`0`
        (if (== (`KismetMathLibrary.RandomIntegerInRange` 0 (`self.Probability_of_pale`)) 0)
          (bind _returnvalue (`|SpawnActorFromClass` "/Game/Blueprints/Zenny/pale_zenny_bounce_BP.pale_zenny_bounce_BP_C" (`self.random_loc_in_circle`) "Undefined" "OverrideRootScale" null null))
          (`PrimitiveComponent.AddImpulse` (`/Game/Blueprints/Zenny/zenny_bounce_BP.StaticMesh` _returnvalue) (`self.disperal_spread`) "None" false)))
      (:`1`
        (if (== (`KismetMathLibrary.RandomIntegerInRange` 0 (`self.probability_of_green`)) 0)
          (bind _returnvalue_2 (`|SpawnActorFromClass` "/Game/Blueprints/Zenny/green_zenny_bounce_BP.green_zenny_bounce_BP_C" (`self.random_loc_in_circle`) "Undefined" "OverrideRootScale" null null))
          (`PrimitiveComponent.AddImpulse` (`/Game/Blueprints/Zenny/zenny_bounce_BP.StaticMesh` _returnvalue_2) (`self.disperal_spread`) "None" false)))
      (:`2`
        (if (== (`KismetMathLibrary.RandomIntegerInRange` 0 (`self.probabilty_of_pink`)) 0)
          (bind _returnvalue_3 (`|SpawnActorFromClass` "/Game/Blueprints/Zenny/pink_zenny_bounce_BP.pink_zenny_bounce_BP_C" (`self.random_loc_in_circle`) "Undefined" "OverrideRootScale" null null))
          (`PrimitiveComponent.AddImpulse` (`/Game/Blueprints/Zenny/zenny_bounce_BP.StaticMesh` _returnvalue_3) (`self.disperal_spread`) "None" false)))
      (:`3`
        (if (== (`KismetMathLibrary.RandomIntegerInRange` 0 (`self.probabilty_of_purple`)) 0)
          (bind _returnvalue_4 (`|SpawnActorFromClass` "/Game/Blueprints/Zenny/purple_zenny_bounce_BP.purple_zenny_bounce_BP_C" (`self.random_loc_in_circle`) "Undefined" "OverrideRootScale" null null))
          (`PrimitiveComponent.AddImpulse` (`/Game/Blueprints/Zenny/zenny_bounce_BP.StaticMesh` _returnvalue_4) (`self.disperal_spread`) "None" false)))))
  ;[1 1 1] Orange Cube Drops
  (if (> (`self.amount_of_cubes_to_drop`) 0)
    (for _ (range 1 (+ (`self.amount_of_cubes_to_drop`) 1))
      (bind _returnvalue_5 (`|SpawnActorFromClass` "/Game/Blueprints/Items/OrangeEnergyCubeBP.OrangeEnergyCubeBP_C" (`self.random_loc_in_circle`) "Undefined" "OverrideRootScale" null null))
      (`PrimitiveComponent.AddImpulse` (`/Game/Blueprints/Items/OrangeEnergyCubeBP.StaticMesh` _returnvalue_5) (`self.disperal_spread`) "None" false)))
  (`self.K2_DestroyActor`))

(event `self.ReceiveBeginPlay`)

(fn `UserConstructionScript`)