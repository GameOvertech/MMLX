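; BP_Door is a sliding double door that the player, identified by the MegamanCapsule tag, opens with the Interact input.
; Its trigger volume enables input and tracks proximity, and leaving the volume closes an opened door automatically.
; One timeline slides both panels along Y, playing forward to open and in reverse to close, each with a sound.
; DoOnce gates and state flags guard against repeated triggering.
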(event `InputAction|Interact`
  (params (Key :type "Key Structure"))
  ;[1 1 1] Door Open/Close
  (:`Pressed`
    (set `self.Interact` true)
    (if (and (`self.Interact`) (`self.NearDoor`)) :!label _label
      (set `self.Interact` false)
      (set `self.DoorClosed` false)
      (`/Engine/EditorBlueprintResources/StandardMacros.DoOnce` false :!label _label_2
        (:`Completed`
          (`GameplayStatics.SpawnSound2D` "/Game/Audio/SFX/sfx_general/sfx-ruindoor-open1.sfx-ruindoor-open1")
          (bind (_direction _doorleft_slide _doorright_slide) (`Timeline|DoorMovement` :!via `PlayFromStart` :!label _label_3)
            (:`Update`
              (`|ExecutionSequence`
                (:`then_0`
                  (`SceneComponent.K2_SetRelativeTransform` (`self.DoorLeft_01`) (`KismetMathLibrary.MakeTransform` (`KismetMathLibrary.MakeVector` 0.0 (.y (.location (`KismetMathLibrary.MakeTransform` (`KismetMathLibrary.MakeVector` 0.0 _doorright_slide))))) (struct) (0.25 1.75 4.25)) false false))
                (:`then_1`
                  (`SceneComponent.K2_SetRelativeTransform` (`self.DoorRight_01`) (`KismetMathLibrary.MakeTransform` (`KismetMathLibrary.MakeVector` 0.0 (.y (.location (`KismetMathLibrary.MakeTransform` (`KismetMathLibrary.MakeVector` 0.0 _doorleft_slide))))) (struct) (0.25 1.75 4.25)) false false))))
            (:`Finished`
              (if (`self.DoorClosed`)
                (goto _label_2 :!via `Reset`))))))
      (else
        (set `self.Interact` false)
        (goto _label_4 :!via `Reset`)))))

(event `self.DoorTrigger.OnComponentBeginOverlap`
  (params (OverlappedComponent :type "PrimitiveComponent Object Reference") (OtherActor :type "Actor Object Reference") (OtherComp :type "PrimitiveComponent Object Reference") (OtherBodyIndex :type Integer) (bFromSweep :type Boolean) (SweepResult :type "HitResult Structure (by ref)"))
  ;[1 1 1] Door Open/Close
  (if (`ActorComponent.ComponentHasTag` OtherComp "MegamanCapsule")
    (`self.EnableInput` (`GameplayStatics.GetPlayerController` 0))
    (set `self.NearDoor` true)
    (goto _label)))

(event `self.DoorTrigger.OnComponentEndOverlap`
  (params (OverlappedComponent :type "PrimitiveComponent Object Reference") (OtherActor :type "Actor Object Reference") (OtherComp :type "PrimitiveComponent Object Reference") (OtherBodyIndex :type Integer))
  ;[1 1 1] Door Open/Close
  (if (`ActorComponent.ComponentHasTag` OtherComp "MegamanCapsule")
    (`self.DisableInput` (`GameplayStatics.GetPlayerController` 0))
    (set `self.NearDoor` false)
    (if (not (`self.DoorClosed`))
      (set `self.NearDoor` false)
      (set `self.DoorClosed` true)
      (`/Engine/EditorBlueprintResources/StandardMacros.DoOnce` false :!label _label_4
        (:`Completed`
          (`GameplayStatics.SpawnSound2D` "/Game/Audio/SFX/sfx_general/sfx-ruindoor-close1.sfx-ruindoor-close1")
          (goto _label_3 :!via `ReverseFromEnd`))))))

(fn `UserConstructionScript`)